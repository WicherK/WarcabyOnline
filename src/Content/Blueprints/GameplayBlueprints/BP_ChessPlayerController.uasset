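; Player controller for a chess match that manages the local player's match screens and mouse input.
; On BeginPlay it enables cursor and game-and-UI input, pauses the game instance's music and binds to match start and end events.
; The pre-match event shows the opponent's nickname and creates the pause menu that Escape toggles.
; The end-game event shows a screen with result, experience and opponent nickname; both events act only on the local controller.
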(event `self.ReceiveBeginPlay`
  (set `self.bShowMouseCursor` true)
  (`WidgetBlueprintLibrary.SetInputMode_GameAndUIEx` self null "DoNotLock" false)
  (bind _asbp_game_instnace (cast `/Game/Blueprints/GameplayBlueprints/BP_GameInstnace` (`GameplayStatics.GetGameInstance`)))
  (`/Game/Blueprints/GameplayBlueprints/BP_GameInstnace.PauseMusic` _asbp_game_instnace)
  (add `self.ShowBeforeMatchScreen` (delegate `ShowBeforeMatchScreenEvent`))
  (add `self.OnEndGame` (delegate `OnEndGameEvent`)))

(event `ShowBeforeMatchScreenEvent`
  (if (`self.IsLocalPlayerController`)
    (bind _returnvalue (`|CreateWidget` "/Game/Blueprints/UI/WBP_BeforeMatchScreen.WBP_BeforeMatchScreen_C" self))
    (`/Game/Blueprints/UI/WBP_BeforeMatchScreen.SetEnemyNickname` _returnvalue (`self.enemyNickname`))
    (`UserWidget.AddToViewport` _returnvalue 0)
    (bind _returnvalue_2 (`|CreateWidget` "/Game/Blueprints/UI/WBP_PauseMenu.WBP_PauseMenu_C"))
    (`UserWidget.AddToViewport` _returnvalue_2 0)
    (set `self.WBP_PauseMenu` _returnvalue_2)))

(event `Key|Escape`
  (params (Key :type "Key Structure"))
  (:`Pressed`
    (`/Game/Blueprints/UI/WBP_PauseMenu.TogglePauseMenu` (`self.WBP_PauseMenu`))))

(event `OnEndGameEvent`
  (params (isWin :type Boolean) (isOvertime :type Boolean) (isSurrender :type Boolean) (expAfterMatch :type Integer))
  (if (`self.IsLocalPlayerController`)
    (bind _returnvalue (`|CreateWidget` "/Game/Blueprints/UI/WBP_EndGameScreen.WBP_EndGameScreen_C" self))
    (`/Game/Blueprints/UI/WBP_EndGameScreen.SetWin` _returnvalue isWin isOvertime isSurrender)
    (`/Game/Blueprints/UI/WBP_EndGameScreen.SetExp` _returnvalue expAfterMatch)
    (`/Game/Blueprints/UI/WBP_EndGameScreen.SetEnemyNickname` _returnvalue (`self.enemyNickname`))
    (`UserWidget.AddToViewport` _returnvalue 0)))

(fn `UserConstructionScript`)