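; Game instance Blueprint that controls a single background music track for the game.
; PlayMusic resumes the stored audio component if valid, otherwise spawns a quiet 2D sound that persists across level transitions and does not auto-destroy.
; PauseMusic and SetVolume act on that same stored component after a validity check, and the Init event is empty.
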(event `self.ReceiveInit`)

(fn `PauseMusic`
  (bind _music (`self.music`))
  (`/Engine/EditorBlueprintResources/StandardMacros.IsValid` _music
    (:`Is Valid`
      (`AudioComponent.SetPaused` _music true))))

(fn `PlayMusic`
  (bind _music (`self.music`))
  (`/Engine/EditorBlueprintResources/StandardMacros.IsValid` _music
    (:`Is Valid`
      (`AudioComponent.SetPaused` _music false))
    (:`Is Not Valid`
      (bind _returnvalue (`GameplayStatics.SpawnSound2D` "/Game/Assets/Music/02__Stonefire.02__Stonefire" 0.1 1.0 0.0 null true false))
      (set `self.music` _returnvalue))))

(fn `SetVolume`
  (params (VolumeMultiplier :type "Float (double-precision)"))
  (bind _music (`self.music`))
  (`/Engine/EditorBlueprintResources/StandardMacros.IsValid` _music
    (:`Is Valid`
      (`AudioComponent.SetVolumeMultiplier` _music VolumeMultiplier))))