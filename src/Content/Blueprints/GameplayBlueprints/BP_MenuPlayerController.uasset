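; Player controller for the menu, handling the Play and Settings button actions.
; On BeginPlay it adds the settings and game-search widgets to the viewport, shows the cursor with Game and UI input, and views through a CineCameraActor found in the level.
; Play shows the searching screen and starts matchmaking through the multiplayer subsystem's FindGame, while Settings opens the menu settings widget.
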(event `self.ReceiveBeginPlay`
  (`WidgetBlueprintLibrary.SetHardwareCursor` "Default" "Default")
  (`UserWidget.AddToViewport` (`self.WBP_SettingsWidget`) 0)
  (`UserWidget.AddToViewport` (`self.WBP_SearchGameWidget`) 0)
  (set `self.bShowMouseCursor` true)
  (`WidgetBlueprintLibrary.SetInputMode_GameAndUIEx` self null "DoNotLock" false)
  (bind _returnvalue (`GameplayStatics.GetActorOfClass` "/Script/CinematicCamera.CineCameraActor"))
  (`self.SetViewTargetWithBlend` _returnvalue)
  (`WidgetBlueprintLibrary.SetHardwareCursor` "Default" "Default"))

(fn `OnPlayButtonClicked`
  (bind _aswbp_searching_game (cast `/Game/Blueprints/UI/WBP_SearchingGame` (`self.WBP_SearchGameWidget`)))
  (`/Game/Blueprints/UI/WBP_SearchingGame.ToggleSearchingScreen` _aswbp_searching_game true)
  (`MultiplayerSubsystem.FindGame` (subsystem `MultiplayerSubsystem`)))

(fn `OnSettingsButtonClicked`
  (bind _aswbp_menu_settings (cast `/Game/Blueprints/UI/WBP_MenuSettings` (`self.WBP_SettingsWidget`)))
  (`/Game/Blueprints/UI/WBP_MenuSettings.ToggleMenuSettings` _aswbp_menu_settings true))

(fn `UserConstructionScript`)