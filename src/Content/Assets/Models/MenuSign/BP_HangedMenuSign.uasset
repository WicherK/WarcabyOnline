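; BP_HangedMenuSign is a wooden menu sign hanging from two chains that sways gently in the scene.
; On BeginPlay it binds the sign to the attachment component of its left and right BP_Chain child actors through two physics constraints.
; Each tick it adds a sideways force along Y that follows a cosine of elapsed time, producing a continuous physics-driven swing.
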(event `self.ReceiveBeginPlay`
  (bind _asbp_chain (cast `/Game/Assets/Models/Chain/BP_Chain` (`ChildActorComponent.ChildActor` (`self.BP_ChainLeft`))))
  (`PhysicsConstraintComponent.SetConstrainedComponents` (`self.LeftConstraint`) (`self.WoodMenuSign`) "None" (`/Game/Assets/Models/Chain/BP_Chain.AttachementChain` _asbp_chain) "None")
  (bind _asbp_chain_2 (cast `/Game/Assets/Models/Chain/BP_Chain` (`ChildActorComponent.ChildActor` (`self.BP_ChainRight`))))
  (`PhysicsConstraintComponent.SetConstrainedComponents` (`self.RightConstraint`) (`self.WoodMenuSign`) "None" (`/Game/Assets/Models/Chain/BP_Chain.AttachementChain` _asbp_chain_2) "None"))

(event `self.ReceiveTick`
  (params (DeltaSeconds :type "Float (single-precision)"))
  ;[1 1 1] Swing animation
  (set `self.Time` (+ (`self.Time`) DeltaSeconds))
  (`PrimitiveComponent.AddForce` (`self.WoodMenuSign`) (`KismetMathLibrary.MakeVector` 0.0 (* (`KismetMathLibrary.Cos` (`self.Time`)) 100.0)) "None" false))

(fn `UserConstructionScript`)