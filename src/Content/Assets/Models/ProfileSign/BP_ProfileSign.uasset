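; Hanging profile sign actor that shows the local player's nickname, Steam avatar, wins, losses, level, XP bar and rank.
; BeginPlay constrains the sign to two chain child actors and requests player info from the multiplayer subsystem.
; The info callback fetches the avatar, then fills the texts, avatar dynamic material, progress widget and rank-point tier material (600–700 sets none).
; Tick applies a sine-wave force to swing the sign.
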(event `self.ReceiveBeginPlay`
  (bind _returnvalue (subsystem `MultiplayerSubsystem`))
  ;[1 1 1] Attach Chains
  (bind _asbp_chain (cast `/Game/Assets/Models/Chain/BP_Chain` (`ChildActorComponent.ChildActor` (`self.BP_ChainLeft`))))
  (`PhysicsConstraintComponent.SetConstrainedComponents` (`self.PCLeft`) (`self.ProfileSign`) "None" (`/Game/Assets/Models/Chain/BP_Chain.AttachementChain` _asbp_chain) "None")
  (bind _asbp_chain_2 (cast `/Game/Assets/Models/Chain/BP_Chain` (`ChildActorComponent.ChildActor` (`self.BP_ChainRight`))))
  (`PhysicsConstraintComponent.SetConstrainedComponents` (`self.PCRight`) (`self.ProfileSign`) "None" (`/Game/Assets/Models/Chain/BP_Chain.AttachementChain` _asbp_chain_2) "None")
  (add `MultiplayerSubsystem.onPlayerInfoDetails` _returnvalue (delegate `CustomEvent`))
  (`MultiplayerSubsystem.SetPlayerInfo` _returnvalue))

(event `CustomEvent`
  (params (PlayerInfo :type "PlayerInfo Structure"))
  (bind (_playerid _nickname _wins _loses _rankpoints _level _levelpoints _nextlevelpoints) (break `PlayerInfo` PlayerInfo))
  (bind _returnvalue (`AdvancedSteamFriendsLibrary.GetSteamFriendAvatar` (`AdvancedSessionsLibrary.GetUniqueNetIDFromPlayerState` (`GameplayStatics.GetPlayerState` 0)) "SteamAvatar_Large")
    (:`OnSuccess`
      _)
    (:`OnFailure`
      _))
  (`self.ShowProfileInfoOnSign` _nickname _returnvalue _wins _loses _level _levelpoints _nextlevelpoints _rankpoints))

(event `self.ReceiveTick`
  (params (DeltaSeconds :type "Float (single-precision)"))
  ;[1 1 1] Swing animation
  (set `self.Time` (+ (`self.Time`) DeltaSeconds))
  (`PrimitiveComponent.AddForce` (`self.ProfileSign`) (`KismetMathLibrary.MakeVector` 0.0 (* (`KismetMathLibrary.Sin` (`self.Time`)) 100.0)) "None" false))

(fn `ShowProfileInfoOnSign`
  (params (profileName :type String) (avatarTexture :type "Texture2D Object Reference") (wins :type Integer) (loses :type Integer) (level :type Integer) (levelPoints :type Integer) (nextLevelPoints :type Integer) (rankPoints :type Integer))
  (set `self.Rank Points` rankPoints)
  (`TextRenderComponent.K2_SetText` (`self.Nickname`) (`KismetTextLibrary.Conv_StringToText` profileName))
  (bind _returnvalue (`KismetMaterialLibrary.CreateDynamicMaterialInstance` (`PrimitiveComponent.GetMaterial` (`self.avatarmesh`) 0)))
  (`MaterialInstanceDynamic.SetTextureParameterValue` _returnvalue "AvatarTexture" avatarTexture)
  (`PrimitiveComponent.SetMaterial` (`self.avatarmesh`) 0 _returnvalue)
  (`TextRenderComponent.K2_SetText` (`self.WinsText`) (`KismetTextLibrary.Conv_IntToText` wins))
  (`TextRenderComponent.K2_SetText` (`self.LosesText`) (`KismetTextLibrary.Conv_IntToText` loses))
  (`TextRenderComponent.K2_SetText` (`self.LevelText`) (`KismetTextLibrary.Conv_StringToText` (`KismetStringLibrary.Concat_StrStr` "Lv." (`KismetStringLibrary.Conv_IntToString` level))))
  (bind _aswbp_progress_bar (cast `/Game/Assets/Models/ProfileSign/WBP_ProgressBar` (`WidgetComponent.GetUserWidgetObject` (`self.ExpBarWidget`))))
  (`/Game/Assets/Models/ProfileSign/WBP_ProgressBar.SetPercentage` _aswbp_progress_bar (`KismetMathLibrary.Conv_IntToDouble` levelPoints) (`KismetMathLibrary.Conv_IntToDouble` nextLevelPoints))
  (if (`KismetMathLibrary.InRange_IntInt` (`self.Rank Points`) 0 250 true false)
    (`PrimitiveComponent.SetMaterial` (`self.Rank`) 0 (`|GetArrayItem` (`self.RankMaterials`)))
    (elif (`KismetMathLibrary.InRange_IntInt` (`self.Rank Points`) 250 400 true false)
      (`PrimitiveComponent.SetMaterial` (`self.Rank`) 0 (`|GetArrayItem` (`self.RankMaterials`) 1))
      (elif (`KismetMathLibrary.InRange_IntInt` (`self.Rank Points`) 400 500 true false)
        (`PrimitiveComponent.SetMaterial` (`self.Rank`) 0 (`|GetArrayItem` (`self.RankMaterials`) 2))
        (elif (`KismetMathLibrary.InRange_IntInt` (`self.Rank Points`) 500 600 true false)
          (`PrimitiveComponent.SetMaterial` (`self.Rank`) 0 (`|GetArrayItem` (`self.RankMaterials`) 3))
          (elif (> (`self.Rank Points`) 700)
            (`PrimitiveComponent.SetMaterial` (`self.Rank`) 0 (`|GetArrayItem` (`self.RankMaterials`) 4))))))))

(fn `UserConstructionScript`)