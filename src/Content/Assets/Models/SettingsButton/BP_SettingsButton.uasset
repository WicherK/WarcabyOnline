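; BP_SettingsButton is a 3D menu settings button that hangs from two chains and forwards clicks to the menu player controller.
; On BeginPlay, physics constraints link the button mesh to the attachment chain of each child BP_ChainShorter actor.
; Tick applies a time-based cosine force along Y to keep the button swinging.
; Clicking it calls OnSettingsButtonClicked on BP_MenuPlayerController.
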(event `self.ReceiveBeginPlay`
  (bind _asbp_chain_shorter (cast `/Game/Assets/Models/Chain/BP_ChainShorter` (`ChildActorComponent.ChildActor` (`self.BP_ChainShorterLeft`))))
  (`PhysicsConstraintComponent.SetConstrainedComponents` (`self.PC_Left`) (`self.SettingsButton`) "None" (`/Game/Assets/Models/Chain/BP_ChainShorter.AttachementChain` _asbp_chain_shorter) "None")
  (bind _asbp_chain_shorter_2 (cast `/Game/Assets/Models/Chain/BP_ChainShorter` (`ChildActorComponent.ChildActor` (`self.BP_ChainShorterRight`))))
  (`PhysicsConstraintComponent.SetConstrainedComponents` (`self.PC_Right`) (`self.SettingsButton`) "None" (`/Game/Assets/Models/Chain/BP_ChainShorter.AttachementChain` _asbp_chain_shorter_2) "None"))

(event `self.ReceiveTick`
  (params (DeltaSeconds :type "Float (single-precision)"))
  ;[1 1 1] Swing animation
  (set `self.Time` (+ (`self.Time`) DeltaSeconds))
  (`PrimitiveComponent.AddForce` (`self.SettingsButton`) (`KismetMathLibrary.MakeVector` 0.0 (* (`KismetMathLibrary.Cos` (/ (`self.Time`) 1.4)) 100.0)) "None" false))

(event `self.SettingsButton.OnClicked`
  (params (TouchedComponent :type "PrimitiveComponent Object Reference") (ButtonPressed :type "Key Structure"))
  (bind _asbp_menu_player_controller (cast `/Game/Blueprints/GameplayBlueprints/BP_MenuPlayerController` (`GameplayStatics.GetPlayerController` 0)))
  (`/Game/Blueprints/GameplayBlueprints/BP_MenuPlayerController.OnSettingsButtonClicked` _asbp_menu_player_controller))

(fn `UserConstructionScript`)