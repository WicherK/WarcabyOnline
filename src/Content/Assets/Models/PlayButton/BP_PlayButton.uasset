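; BP_PlayButton is a clickable menu play button actor that hangs from two chains and sways.
; BeginPlay binds the button to the attachment component of each child BP_Chain actor through left and right physics constraints.
; Tick pushes it with a time-based sine force along Y for the swing.
; Clicking forwards to BP_MenuPlayerController's OnPlayButtonClicked, while the cursor hover events are empty.
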(event `self.ReceiveBeginPlay`
  (bind _asbp_chain (cast `/Game/Assets/Models/Chain/BP_Chain` (`ChildActorComponent.ChildActor` (`self.BP_ChainLeft`))))
  (`PhysicsConstraintComponent.SetConstrainedComponents` (`self.PCLeft`) (`self.PlayButton`) "None" (`/Game/Assets/Models/Chain/BP_Chain.AttachementChain` _asbp_chain) "None")
  (bind _asbp_chain_2 (cast `/Game/Assets/Models/Chain/BP_Chain` (`ChildActorComponent.ChildActor` (`self.BP_ChainRight`))))
  (`PhysicsConstraintComponent.SetConstrainedComponents` (`self.PCRight`) (`self.PlayButton`) "None" (`/Game/Assets/Models/Chain/BP_Chain.AttachementChain` _asbp_chain_2) "None"))

(event `self.ReceiveTick`
  (params (DeltaSeconds :type "Float (single-precision)"))
  ;[1 1 1] Swing animation
  (set `self.Time` (+ (`self.Time`) DeltaSeconds))
  (`PrimitiveComponent.AddForce` (`self.PlayButton`) (`KismetMathLibrary.MakeVector` 0.0 (* (`KismetMathLibrary.Sin` (/ (`self.Time`) 1.4)) 150.0)) "None" false))

(event `self.PlayButton.OnClicked`
  (params (TouchedComponent :type "PrimitiveComponent Object Reference") (ButtonPressed :type "Key Structure"))
  (bind _asbp_menu_player_controller (cast `/Game/Blueprints/GameplayBlueprints/BP_MenuPlayerController` (`GameplayStatics.GetPlayerController` 0)))
  (`/Game/Blueprints/GameplayBlueprints/BP_MenuPlayerController.OnPlayButtonClicked` _asbp_menu_player_controller))

(event `self.PlayButton.OnBeginCursorOver`
  (params (TouchedComponent :type "PrimitiveComponent Object Reference")))

(event `self.PlayButton.OnEndCursorOver`
  (params (TouchedComponent :type "PrimitiveComponent Object Reference")))

(fn `UserConstructionScript`)